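; BP_Button is a button actor that can be revealed and pressed to trigger particle effects.
; It disables collision at BeginPlay, and the Buttonvisible event unhides it and turns collision on.
; The buttonPress event runs a DoOnce-guarded timeline that moves the button mesh's relative Z.
; When the timeline finishes, it resets the guard and activates four Niagara components.
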(event `self.ReceiveBeginPlay`
  (`self.SetActorEnableCollision` false))

(event `Button visible`
  (`self.SetActorHiddenInGame` false)
  (`self.SetActorEnableCollision` true))

(event `buttonPress`
  (`/Engine/EditorBlueprintResources/StandardMacros.DoOnce` false :!label _label
    (:`Completed`
      (bind (_direction _newtrack_0) (`Timeline|Button Press` :!via `PlayFromStart`)
        (:`Update`
          (`SceneComponent.K2_SetRelativeLocation` (`self.Buuton3`) (`KismetMathLibrary.MakeVector` 0.0 0.0 _newtrack_0) false false))
        (:`Finished`
          (`|ExecutionSequence`
            (:`then_0`
              (goto _label :!via `Reset`))
            (:`then_1`
              (`ActorComponent.Activate` (`self.Niagara`) false)
              (`ActorComponent.Activate` (`self.Niagara1`) false)
              (`ActorComponent.Activate` (`self.Niagara2`) false)
              (`ActorComponent.Activate` (`self.Niagara3`) false))))))))

(fn `UserConstructionScript`)