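; BP_Room is a room Blueprint that switches numbered static mesh components to set up its look and right-door state.
; On BeginPlay it hides StaticMesh101 and disables its collision, also toggling two other meshes in the Menu level.
; Outside Menu it ends on a Delay with nothing after it.
; The DoorRightHidden event toggles StaticMesh38 and StaticMesh101 visibility and gives the latter query-only collision.
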(event `self.ReceiveBeginPlay`
  (bind _staticmesh101 (`self.StaticMesh101`))
  (bind _staticmesh101_2 (`self.StaticMesh101`))
  (bind _returnvalue (`GameplayStatics.GetCurrentLevelName` true))
  (if (`KismetStringLibrary.EqualEqual_StrStr` _returnvalue "Menu")
    (`SceneComponent.ToggleVisibility` (`self.StaticMesh37`) false)
    (`SceneComponent.ToggleVisibility` (`self.StaticMesh151`) false)
    (`SceneComponent.SetVisibility` _staticmesh101 false false)
    (`PrimitiveComponent.SetCollisionEnabled` _staticmesh101 "NoCollision")
    (else
      (`SceneComponent.SetVisibility` _staticmesh101_2 false false)
      (`PrimitiveComponent.SetCollisionEnabled` _staticmesh101_2 "NoCollision")
      (`KismetSystemLibrary.Delay` 10.0))))

(event `DoorRightHidden`
  (bind _staticmesh101 (`self.StaticMesh101`))
  (`SceneComponent.ToggleVisibility` (`self.StaticMesh38`) false)
  (`SceneComponent.ToggleVisibility` _staticmesh101 false)
  (`PrimitiveComponent.SetCollisionEnabled` _staticmesh101 "QueryOnly"))

(fn `UserConstructionScript`)