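; BP_Droite is a trigger that sends the player to the next right-hand level in a branching level sequence.
; On its first box overlap, it increments RightCounter and records the current level as LastLevel in BP_GameInstance.
; A name-based branch chain picks the destination event, which calls TransitionLevel on the FirstPersonCharacter, waits briefly, then opens that level.
; The event named E_D_Gauche actually opens E_D_Droite.
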(event `Right_A_01`
  ;[1 1 1] Right_A_01
  (bind _asfirst_person_character (cast `/Game/Blueprint/FirstPersonCharacter` (`GameplayStatics.GetPlayerCharacter` 0)))
  (`/Game/Blueprint/FirstPersonCharacter.Transition Level` _asfirst_person_character)
  (`KismetSystemLibrary.Delay` 2.0)
  (`GameplayStatics.OpenLevel` "Right_A_01"))

(event `B_D_Droite`
  ;[1 1 1] B_D_Droite
  (bind _asfirst_person_character (cast `/Game/Blueprint/FirstPersonCharacter` (`GameplayStatics.GetPlayerCharacter` 0)))
  (`/Game/Blueprint/FirstPersonCharacter.Transition Level` _asfirst_person_character)
  (`KismetSystemLibrary.Delay` 2.0)
  (`GameplayStatics.OpenLevel` "B_D_Droite"))

(event `C_D_Droite`
  ;[1 1 1] C_D_Droite
  (bind _asfirst_person_character (cast `/Game/Blueprint/FirstPersonCharacter` (`GameplayStatics.GetPlayerCharacter` 0)))
  (`/Game/Blueprint/FirstPersonCharacter.Transition Level` _asfirst_person_character)
  (`KismetSystemLibrary.Delay` 2.0)
  (`GameplayStatics.OpenLevel` "C_D_Droite"))

(event `D_D_Droite`
  ;[1 1 1] D_D_Droite
  (bind _asfirst_person_character (cast `/Game/Blueprint/FirstPersonCharacter` (`GameplayStatics.GetPlayerCharacter` 0)))
  (`/Game/Blueprint/FirstPersonCharacter.Transition Level` _asfirst_person_character)
  (`KismetSystemLibrary.Delay` 2.0)
  (`GameplayStatics.OpenLevel` "D_D_Droite"))

(event `E_D_Gauche`
  ;[1 1 1] E_D_Gauche
  (bind _asfirst_person_character (cast `/Game/Blueprint/FirstPersonCharacter` (`GameplayStatics.GetPlayerCharacter` 0)))
  (`/Game/Blueprint/FirstPersonCharacter.Transition Level` _asfirst_person_character)
  (`KismetSystemLibrary.Delay` 2.0)
  (`GameplayStatics.OpenLevel` "E_D_Droite"))

(event `F_D_Droite`
  ;[1 1 1] F_D_Droite
  (bind _asfirst_person_character (cast `/Game/Blueprint/FirstPersonCharacter` (`GameplayStatics.GetPlayerCharacter` 0)))
  (`/Game/Blueprint/FirstPersonCharacter.Transition Level` _asfirst_person_character)
  (`KismetSystemLibrary.Delay` 2.0)
  (`GameplayStatics.OpenLevel` "F_D_Droite"))

(event `self.Box.OnComponentBeginOverlap`
  (params (OverlappedComponent :type "PrimitiveComponent Object Reference") (OtherActor :type "Actor Object Reference") (OtherComp :type "PrimitiveComponent Object Reference") (OtherBodyIndex :type Integer) (bFromSweep :type Boolean) (SweepResult :type "HitResult Structure (by ref)"))
  (bind _concurrentlevel (`self.ConcurrentLevel`))
  (bind _concurrentlevel_2 (`self.ConcurrentLevel`))
  (bind _gameinstance (`self.GameInstance`))
  (bind _concurrentlevel_3 (`self.ConcurrentLevel`))
  (`/Engine/EditorBlueprintResources/StandardMacros.DoOnce` false
    (:`Completed`
      (bind _asbp_game_instance (cast `/Game/BP_GameInstance` (`GameplayStatics.GetGameInstance`)))
      (set `self.GameInstance` _asbp_game_instance)
      (bind _returnvalue (`GameplayStatics.GetCurrentLevelName` true))
      (set `self.ConcurrentLevel` _returnvalue)
      (`|ExecutionSequence`
        (:`then_0`
          ;[1 1 1] CounterUp
          (set `/Game/BP_GameInstance.RightCounter` (+ (`/Game/BP_GameInstance.RightCounter` _gameinstance) 1) _gameinstance)
          (set `/Game/BP_GameInstance.Last Level` (`self.ConcurrentLevel`) (`self.GameInstance`)))
        (:`then_1`
          (if (`KismetStringLibrary.EqualEqual_StrStr` (`self.ConcurrentLevel`) "FirstPersonExampleMap")
            (`self.Right_A_01`)
            (elif (or (`KismetStringLibrary.EqualEqual_StrStr` _concurrentlevel_3 "Right_A_01") (`KismetStringLibrary.EqualEqual_StrStr` _concurrentlevel_3 "Left_A_01"))
              (`self.B_D_Droite`)
              (elif (`KismetStringLibrary.EqualEqual_StrStr` (`self.ConcurrentLevel`) "B_D_Droite")
                (`self.C_D_Droite`)
                (elif (or (`KismetStringLibrary.EqualEqual_StrStr` _concurrentlevel "C_D_Gauche") (`KismetStringLibrary.EqualEqual_StrStr` _concurrentlevel "C_D_Droite") (`KismetStringLibrary.EqualEqual_StrStr` _concurrentlevel "C_D_Milieu"))
                  (`self.D_D_Droite`)
                  (elif (or (`KismetStringLibrary.EqualEqual_StrStr` _concurrentlevel_2 "D_D_Droite") (`KismetStringLibrary.EqualEqual_StrStr` _concurrentlevel_2 "D_D_Gauche"))
                    (`self.E_D_Gauche`)
                    (elif (`KismetStringLibrary.EqualEqual_StrStr` (`self.ConcurrentLevel`) "E_D_Droite")
                      (`self.F_D_Droite`))))))))))))

(fn `UserConstructionScript`)