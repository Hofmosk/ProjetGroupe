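; BP_Milieu is a trigger actor that moves the player on to the C_D_Milieu level.
; The first overlap of its Box fires a DoOnce that caches the game instance and reads the current level name.
; If that level is B_D_Gauche or B_D_Droite, it calls the first-person character's TransitionLevel, waits briefly, then opens C_D_Milieu.
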(event `C_D_Milieu`
  ;[1 1 1] C_D_Milieu
  (bind _asfirst_person_character (cast `/Game/Blueprint/FirstPersonCharacter` (`GameplayStatics.GetPlayerCharacter` 0)))
  (`/Game/Blueprint/FirstPersonCharacter.Transition Level` _asfirst_person_character)
  (`KismetSystemLibrary.Delay` 2.0)
  (`GameplayStatics.OpenLevel` "C_D_Milieu"))

(event `self.Box.OnComponentBeginOverlap`
  (params (OverlappedComponent :type "PrimitiveComponent Object Reference") (OtherActor :type "Actor Object Reference") (OtherComp :type "PrimitiveComponent Object Reference") (OtherBodyIndex :type Integer) (bFromSweep :type Boolean) (SweepResult :type "HitResult Structure (by ref)"))
  (bind _concurrent_level (`self.Concurrent_Level`))
  (`/Engine/EditorBlueprintResources/StandardMacros.DoOnce` false
    (:`Completed`
      (bind _asbp_game_instance (cast `/Game/BP_GameInstance` (`GameplayStatics.GetGameInstance`)))
      (set `self.GameInsteance` _asbp_game_instance)
      (bind _returnvalue (`GameplayStatics.GetCurrentLevelName` true))
      (set `self.Concurrent_Level` _returnvalue)
      (if (or (`KismetStringLibrary.EqualEqual_StrStr` _concurrent_level "B_D_Gauche") (`KismetStringLibrary.EqualEqual_StrStr` _concurrent_level "B_D_Droite"))
        (`self.C_D_Milieu`)))))

(fn `UserConstructionScript`)