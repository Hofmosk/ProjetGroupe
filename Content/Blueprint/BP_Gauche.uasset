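; BP_Gauche is a trigger actor for the left-hand path that sends the player to the next level in a branching sequence.
; Its box overlap fires once, increments LeftCounter and records LastLevel in BP_GameInstance.
; A nested name check on the current level picks one of six events, each calling the character's TransitionLevel, then opening a hardcoded level two seconds later.
; Destination suffixes vary between Gauche and Droite, and B_D_Gauche opens B_D_Droite.
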(event `Left_A_01`
  ;[1 1 1] Left_A_01
  (bind _asfirst_person_character (cast `/Game/Blueprint/FirstPersonCharacter` (`GameplayStatics.GetPlayerCharacter` 0)))
  (`/Game/Blueprint/FirstPersonCharacter.Transition Level` _asfirst_person_character)
  (`KismetSystemLibrary.Delay` 2.0)
  (`GameplayStatics.OpenLevel` "Left_A_01"))

(event `B_D_Gauche`
  ;[1 1 1] B_D_Gauche
  (bind _asfirst_person_character (cast `/Game/Blueprint/FirstPersonCharacter` (`GameplayStatics.GetPlayerCharacter` 0)))
  (`/Game/Blueprint/FirstPersonCharacter.Transition Level` _asfirst_person_character)
  (`KismetSystemLibrary.Delay` 2.0)
  (`GameplayStatics.OpenLevel` "B_D_Droite"))

(event `C_D_Droite`
  ;[1 1 1] C_D_Droite
  (bind _asfirst_person_character (cast `/Game/Blueprint/FirstPersonCharacter` (`GameplayStatics.GetPlayerCharacter` 0)))
  (`/Game/Blueprint/FirstPersonCharacter.Transition Level` _asfirst_person_character)
  (`KismetSystemLibrary.Delay` 2.0)
  (`GameplayStatics.OpenLevel` "C_D_Droite"))

(event `D_D_Gauche`
  ;[1 1 1] D_D_Gauche
  (bind _asfirst_person_character (cast `/Game/Blueprint/FirstPersonCharacter` (`GameplayStatics.GetPlayerCharacter` 0)))
  (`/Game/Blueprint/FirstPersonCharacter.Transition Level` _asfirst_person_character)
  (`KismetSystemLibrary.Delay` 2.0)
  (`GameplayStatics.OpenLevel` "D_D_Gauche"))

(event `E_D_Droite`
  ;[1 1 1] E_D_Droite
  (bind _asfirst_person_character (cast `/Game/Blueprint/FirstPersonCharacter` (`GameplayStatics.GetPlayerCharacter` 0)))
  (`/Game/Blueprint/FirstPersonCharacter.Transition Level` _asfirst_person_character)
  (`KismetSystemLibrary.Delay` 2.0)
  (`GameplayStatics.OpenLevel` "E_D_Droite"))

(event `F_D_Gauche`
  ;[1 1 1] F_D_Gauche
  (bind _asfirst_person_character (cast `/Game/Blueprint/FirstPersonCharacter` (`GameplayStatics.GetPlayerCharacter` 0)))
  (`/Game/Blueprint/FirstPersonCharacter.Transition Level` _asfirst_person_character)
  (`KismetSystemLibrary.Delay` 2.0)
  (`GameplayStatics.OpenLevel` "F_D_Gauche"))

(event `self.ReceiveBeginPlay`
  (bind _asbp_game_instance (cast `/Game/BP_GameInstance` (`GameplayStatics.GetGameInstance`)))
  (set `self.GameInstance` _asbp_game_instance))

(event `self.Box.OnComponentBeginOverlap`
  (params (OverlappedComponent :type "PrimitiveComponent Object Reference") (OtherActor :type "Actor Object Reference") (OtherComp :type "PrimitiveComponent Object Reference") (OtherBodyIndex :type Integer) (bFromSweep :type Boolean) (SweepResult :type "HitResult Structure (by ref)"))
  (bind _concurrent_level (`self.Concurrent_Level`))
  (bind _gameinstance (`self.GameInstance`))
  (bind _concurrent_level_2 (`self.Concurrent_Level`))
  (`/Engine/EditorBlueprintResources/StandardMacros.DoOnce` false
    (:`Completed`
      (bind _returnvalue (`GameplayStatics.GetCurrentLevelName` true))
      (set `self.Concurrent_Level` _returnvalue)
      (`|ExecutionSequence`
        (:`then_0`
          (bind _output_get (set `self.GameInstance` _gameinstance))
          (set `/Game/BP_GameInstance.LeftCounter` (+ (`/Game/BP_GameInstance.LeftCounter` _gameinstance) 1) _output_get)
          (set `/Game/BP_GameInstance.Last Level` (`self.Concurrent_Level`) (`self.GameInstance`)))
        (:`then_1`
          (if (`KismetStringLibrary.EqualEqual_StrStr` (`self.Concurrent_Level`) "FirstPersonExampleMap")
            (`self.Left_A_01`)
            (elif (`KismetStringLibrary.EqualEqual_StrStr` (`self.Concurrent_Level`) "Left_A_01")
              (`self.Left_A_01`)
              (elif (`KismetStringLibrary.EqualEqual_StrStr` (`self.Concurrent_Level`) "Right_A_01")
                (`self.B_D_Gauche`)
                (elif (`KismetStringLibrary.EqualEqual_StrStr` (`self.Concurrent_Level`) "B_D_Droite")
                  (`self.C_D_Droite`)
                  (elif (or (`KismetStringLibrary.EqualEqual_StrStr` _concurrent_level_2 "C_D_Gauche") (`KismetStringLibrary.EqualEqual_StrStr` _concurrent_level_2 "C_D_Droite") (`KismetStringLibrary.EqualEqual_StrStr` _concurrent_level_2 "C_D_Milieu"))
                    (`self.D_D_Gauche`)
                    (elif (or (`KismetStringLibrary.EqualEqual_StrStr` _concurrent_level "D_D_Gauche") (`KismetStringLibrary.EqualEqual_StrStr` _concurrent_level "D_D_Droite"))
                      (`self.E_D_Droite`)
                      (elif (`KismetStringLibrary.EqualEqual_StrStr` (`self.Concurrent_Level`) "E_D_Droite")
                        (`self.F_D_Gauche`)))))))))))))

(fn `UserConstructionScript`)