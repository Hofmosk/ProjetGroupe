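; BP_DoorG is a door with two leaves, CubeG and CubeD, that swing open in gameplay or in a menu.
; Open_DoorG opens it once with a sound, while DoorMenuOpen replays sound and swing on each call through separate timelines.
; Each leaf has its own timeline, whose ZRotation output scales Angle into relative yaw.
; Hovered swings both leaves by AngleHover, and UnHovered reverses those timelines.
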(event `Open_DoorG`
  (`/Engine/EditorBlueprintResources/StandardMacros.DoOnce` false
    (:`Completed`
      (`GameplayStatics.PlaySound2D` "/Game/Sound/Environnement/Open_Door.Open_Door" 1.0 1.0 0.0 null null)
      (`|ExecutionSequence`
        (:`then_0`
          (bind (_direction _z_rotation) (`Timeline|Door1`)
            (:`Update`
              (`SceneComponent.K2_SetRelativeRotation` (`self.CubeG`) (`KismetMathLibrary.MakeRotator` 0.0 0.0 (* _z_rotation (`self.Angle`))) false false))))
        (:`then_1`
          (bind (_direction_2 _z_rotation_2) (`Timeline|Door2`)
            (:`Update`
              (`SceneComponent.K2_SetRelativeRotation` (`self.CubeD`) (`KismetMathLibrary.MakeRotator` 0.0 0.0 (* _z_rotation_2 (`self.Angle`))) false false))))))))

(event `DoorMenuOpen`
  ;[1 1 1] Menu
  (`GameplayStatics.PlaySound2D` "/Game/Sound/Environnement/Open_Door.Open_Door" 1.0 1.0 0.0 null null)
  (`|ExecutionSequence`
    (:`then_0`
      (bind (_direction _z_rotation) (`Timeline|Timeline_0`)
        (:`Update`
          (`SceneComponent.K2_SetRelativeRotation` (`self.CubeG`) (`KismetMathLibrary.MakeRotator` 0.0 0.0 (* _z_rotation (`self.Angle`))) false false))))
    (:`then_1`
      (bind (_direction_2 _z_rotation_2) (`Timeline|Timeline_1`)
        (:`Update`
          (`SceneComponent.K2_SetRelativeRotation` (`self.CubeD`) (`KismetMathLibrary.MakeRotator` 0.0 0.0 (* _z_rotation_2 (`self.Angle`))) false false))))))

(event `Hovered`
  ;[1 1 1] Menu
  (`|ExecutionSequence`
    (:`then_0`
      (bind (_direction _z_rotation) (`Timeline|Timeline_2` :!label _label)
        (:`Update`
          (`SceneComponent.K2_SetRelativeRotation` (`self.CubeG`) (`KismetMathLibrary.MakeRotator` 0.0 0.0 (* _z_rotation (`self.Angle_Hover`))) false false))))
    (:`then_1`
      (bind (_direction_2 _z_rotation_2) (`Timeline|Timeline_3` :!label _label_2)
        (:`Update`
          (`SceneComponent.K2_SetRelativeRotation` (`self.CubeD`) (`KismetMathLibrary.MakeRotator` 0.0 0.0 (* _z_rotation_2 (`self.Angle_Hover`))) false false))))))

(event `UnHovered`
  ;[1 1 1] Menu
  (`|ExecutionSequence`
    (:`then_0`
      (goto _label :!via `Reverse`))
    (:`then_1`
      (goto _label_2 :!via `Reverse`))))

(fn `UserConstructionScript`)